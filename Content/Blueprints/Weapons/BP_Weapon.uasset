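; Weapon actor that a character can pick up, drop and fire, with all three actions gated on server authority.
; Pickup records the character and player number and attaches the weapon through the character, while Drop detaches it at the character's location.
; Shoot checks ammo and a CanShoot flag, calls ShootLogic, spends a round, then blocks firing for the FireRate delay.
; ShootLogic is a separate event that only prints a placeholder message.
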(event `DelayShoot`
  (set `self.bCanShoot` false)
  (`KismetSystemLibrary.Delay` (`self.FireRate`))
  (set `self.bCanShoot` true))

(event `Shoot`
  (if (`self.HasAuthority`)
    (if (`self.bCanShoot`)
      (if (> (`self.Ammo`) 0)
        (`self.ShootLogic`)
        (`/Engine/EditorBlueprintResources/StandardMacros.DecrementInt` (`self.Ammo`)
          (:`  `
            (`self.DelayShoot`)))))))

(event `ShootLogic`
  (`KismetSystemLibrary.PrintString` "Shoot logic"))

(fn `Drop`
  (if (`self.HasAuthority`)
    (if (`self.bIsHeld`)
      (`self.K2_DetachFromActor` "KeepRelative")
      (`self.K2_SetActorLocation` (`self.K2_GetActorLocation` (`self.Character`)))
      (set `self.bIsHeld` false)
      (set `self.Character` null))))

(fn `Pickup`
  (params (Character :type "/Game/Blueprints/Characters/BP_Character Object Reference"))
  (returns (Weapon :type "/Game/Blueprints/Weapons/BP_Weapon Object Reference") (PickedUp :type Boolean))
  (if (`self.HasAuthority`)
    (if (not (`self.bIsHeld`))
      (bind _output_get (set `self.Character` Character))
      (set `self.PlayerNumber` (`/Game/Blueprints/Characters/BP_Character.PlayerNumber` _output_get))
      (`/Game/Blueprints/Characters/BP_Character.AttachWeapon` _output_get self)
      (`self.K2_SetActorRelativeLocation` (0.0 0.0 0.0))
      (set `self.bIsHeld` true)
      (return self true)
      (else
        _)))
  (return null false))

(fn `UserConstructionScript`)