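; Pistol weapon Blueprint that fires a single BP_Bullet each time its ShootLogic event runs.
; The bullet spawns just in front of the Scene component, aligned to that component's axes.
; It is owned by the pistol and receives the player number, initial force, damage and the character's facing direction.
; The file holds no other active logic.
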(event `self.ShootLogic`
  (bind _scene (`self.Scene`))
  (bind _returnvalue (`SceneComponent.GetForwardVector` _scene))
  (`|SpawnActorFromClass` "/Game/Blueprints/Projectiles/BP_Bullet.BP_Bullet_C" (`KismetMathLibrary.MakeTransform` (+ (`SceneComponent.K2_GetComponentLocation` _scene) _returnvalue) (`KismetMathLibrary.MakeRotationFromAxes` _returnvalue (`SceneComponent.GetRightVector` _scene) (`SceneComponent.GetUpVector` _scene))) "Undefined" "OverrideRootScale" self (`self.PlayerNumber`) (`self.InitialForce`) (`self.Damage`) (`/Game/Blueprints/Characters/BP_Character.IsFacingRight` (`self.Character`)) null))

(fn `UserConstructionScript`
  (`parent.UserConstructionScript`))